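; BP_Restart is a trigger actor that restarts the current level when the player pawn enters its Box.
; On overlap it fades the camera to dark red, holds it, and waits out the fade before reopening the current level by name.
; On BeginPlay it fades in from the same color, so the reload reads as a continuous transition.
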(event OnComponentBeginOverlap(Box)
  (params (OverlappedComponent :type Primitive%20Component%20Object%20Reference) (OtherActor :type Actor%20Object%20Reference) (OtherComp :type Primitive%20Component%20Object%20Reference) (OtherBodyIndex :type Integer) (bFromSweep :type Boolean) (SweepResult :type Hit%20Result%20Structure%20%28by%20ref%29))
  (bind _returnvalue (Math|Float|MakeLiteralFloat 1.0))
  (if (== OtherActor (Game|Player|GetPlayerPawn 0))
    (CameraFades|StartCameraFade (Game|GetPlayerCameraManager 0) 0.0 1.0 _returnvalue "(R=0.258333,G=0.000000,B=0.006996,A=1.000000)" false true)
    (Utilities|FlowControl|Delay _returnvalue)
    (bind _returnvalue_2 (Game|GetCurrentLevelName true))
    (Game|OpenLevel(byName) (Utilities|String|StringToName _returnvalue_2))))

(event EventBeginPlay
  (CameraFades|StartCameraFade (Game|GetPlayerCameraManager 0) 1.0 0.0 (Math|Float|MakeLiteralFloat 1.0) "(R=0.258333,G=0.000000,B=0.006996,A=1.000000)" false false))

(fn ConstructionScript)